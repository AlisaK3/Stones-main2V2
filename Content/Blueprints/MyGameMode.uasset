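; Game mode that shows lives and timer widgets and counts elapsed seconds while the player's StonePawner pawn has ButtonPressed set.
; Tick casts player pawn 0 to StonePawner and, while that flag is true, creates new Lives and TimerCount widgets on every frame and adds them to the viewport.
; A one-second Delay within Tick paces the TimeSec increment, acting as a simple seconds counter.
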(event `self.ReceiveTick`
  (params (DeltaSeconds :type "Float (single-precision)"))
  (bind _asstone_pawner (cast `/Game/Blueprints/StonePawner` (`GameplayStatics.GetPlayerPawn` 0)))
  (if (`/Game/Blueprints/StonePawner.Button Pressed` _asstone_pawner)
    (bind _returnvalue (`|CreateWidget` "/Game/Widgets/Lives.Lives_C"))
    (`UserWidget.AddToViewport` _returnvalue 0)
    (bind _returnvalue_2 (`|CreateWidget` "/Game/Widgets/TimerCount.TimerCount_C"))
    (`UserWidget.AddToViewport` _returnvalue_2 0)
    (set `self.TimeSec` (`self.TimeSec`))
    (`KismetSystemLibrary.Delay` 1.0)
    (set `self.TimeSec` (+ (`self.TimeSec`) 1))))

(fn `UserConstructionScript`)