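; Spawn_cube is a cube actor that reacts to overlaps with cube and cube2 actors to change player lives or game time.
; Starting an overlap with cube2 plays audio and hides its mesh.
; The first end overlap, gated by DoOnce, either removes a life for cube or adds time for cube2 through MyGameMode.
; At zero lives it shows the GameOver widget, then reloads FirstLevel after a delay.
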(event `self.ReceiveActorBeginOverlap`
  (params (OtherActor :type "Actor Object Reference"))
  (cast `/Game/Blueprints/cube2` OtherActor)
  (`AddComponent|NODE_AddAudioComponent-3`)
  (`SceneComponent.SetVisibility` (`self.Cube`) false false))

(event `self.ReceiveActorEndOverlap`
  (params (OtherActor :type "Actor Object Reference"))
  (`/Engine/EditorBlueprintResources/StandardMacros.DoOnce` false
    (:`Completed`
      (cast `/Game/Blueprints/cube` OtherActor
        (:`then`
          (`AddComponent|NODE_AddAudioComponent-0`)
          (bind _asmy_game_mode (cast `/Game/Blueprints/MyGameMode` (`GameplayStatics.GetGameMode`)))
          (bind _output_get (set `/Game/Blueprints/MyGameMode.Max Lives` (- (`/Game/Blueprints/MyGameMode.Max Lives` _asmy_game_mode) 1) _asmy_game_mode))
          (if (== _output_get 0)
            (bind _returnvalue (`|CreateWidget` "/Game/Widjets/GameOver.GameOver_C"))
            (`UserWidget.AddToViewport` _returnvalue 0)
            (`self.DisableInput` null)
            (`KismetSystemLibrary.Delay` 2.0)
            (`GameplayStatics.OpenLevel` "FirstLevel")))
        (:`CastFailed`
          (cast `/Game/Blueprints/cube2` OtherActor)
          (`/Engine/EditorBlueprintResources/StandardMacros.DoOnce` false
            (:`Completed`
              (`AddComponent|NODE_AddAudioComponent-2`)
              (bind _asmy_game_mode_2 (cast `/Game/Blueprints/MyGameMode` (`GameplayStatics.GetGameMode`)))
              (set `/Game/Blueprints/MyGameMode.TimeSec` (+ (`/Game/Blueprints/MyGameMode.TimeSec` _asmy_game_mode_2) 10) _asmy_game_mode_2))))))))

(fn `UserConstructionScript`)