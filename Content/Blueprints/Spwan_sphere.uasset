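; Moving sphere collectible that the player catches for score time or misses at the cost of a life.
; A timeline moves it along local Z, at a speed raised at BeginPlay once the game mode's TimeSec reaches 50.
; Overlapping a cube plays the impact effect, flags StonePawner and later adds TimeSec.
; Leaving a cube2 costs a life through DoOnce guards, showing GameOver and reloading FirstLevel at zero.
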(event `ObjectSpeed`
  (bind _asmy_game_mode (cast `/Game/Blueprints/MyGameMode` (`GameplayStatics.GetGameMode`)))
  (if (< (`/Game/Blueprints/MyGameMode.TimeSec` _asmy_game_mode) 50)
    (set `self.Object Speed` (`self.Object Speed`))
    (else
      (set `self.Object Speed` (+ (* (/ (`/Game/Blueprints/MyGameMode.TimeSec` _asmy_game_mode) 50) 2.0) (`self.Object Speed`))))))

(event `self.ReceiveBeginPlay`
  (`SceneComponent.SetVisibility` (`self.Impact`) false false)
  (`self.ObjectSpeed`)
  (`Timeline|Timeline_0`
    (:`Update`
      (`self.K2_AddActorLocalOffset` (`KismetMathLibrary.MakeVector` 0.0 0.0 (* (`self.Object Speed`) (`GameplayStatics.GetWorldDeltaSeconds`)))))))

(event `self.ReceiveActorBeginOverlap`
  (params (OtherActor :type "Actor Object Reference"))
  (bind _impact (`self.Impact`))
  (`|ExecutionSequence`
    (:`then_0`
      (`/Engine/EditorBlueprintResources/StandardMacros.DoOnce` false
        (:`Completed`
          (cast `/Game/Blueprints/cube` OtherActor)
          (`AddComponent|NODE_AddAudioComponent-1`)
          (`SceneComponent.SetVisibility` (`self.Sphere`) false false)
          (`SceneComponent.SetVisibility` _impact true false)
          (`PaperFlipbookComponent.SetPlaybackPositionInFrames` _impact 0 false)
          (`KismetSystemLibrary.Delay` 0.5)
          (`SceneComponent.SetVisibility` (`self.Impact`) false false)
          (`ActorComponent.K2_DestroyComponent` (`self.Impact`))
          (bind _asstone_pawner (cast `/Game/Blueprints/StonePawner` (`GameplayStatics.GetPlayerPawn` 0)))
          (set `/Game/Blueprints/StonePawner.ObjectCollected` true _asstone_pawner))))))

(event `self.ReceiveActorEndOverlap`
  (params (OtherActor :type "Actor Object Reference"))
  (`|ExecutionSequence`
    (:`then_0`
      (cast `/Game/Blueprints/cube` OtherActor)
      (`/Engine/EditorBlueprintResources/StandardMacros.DoOnce` false
        (:`Completed`
          (`KismetSystemLibrary.Delay` 0.2)
          (bind _asmy_game_mode (cast `/Game/Blueprints/MyGameMode` (`GameplayStatics.GetGameMode`)))
          (set `/Game/Blueprints/MyGameMode.TimeSec` (+ (`/Game/Blueprints/MyGameMode.TimeSec` _asmy_game_mode) 10) _asmy_game_mode)
          (bind _asstone_pawner (cast `/Game/Blueprints/StonePawner` (`GameplayStatics.GetPlayerPawn` 0)))
          (set `/Game/Blueprints/StonePawner.ObjectCollected` true _asstone_pawner))))
    (:`then_1`
      (`/Engine/EditorBlueprintResources/StandardMacros.DoOnce` false
        (:`Completed`
          (cast `/Game/Blueprints/cube2` OtherActor)
          (`AddComponent|NODE_AddAudioComponent-0`)
          (`self.MinusLive`)
          (bind _asstone_pawner_2 (cast `/Game/Blueprints/StonePawner` (`GameplayStatics.GetPlayerPawn` 0)))
          (set `/Game/Blueprints/StonePawner.ObjectCollected` false _asstone_pawner_2))))))

(event `MinusLive`
  (`/Engine/EditorBlueprintResources/StandardMacros.DoOnce` false
    (:`Completed`
      (bind _asmy_game_mode (cast `/Game/Blueprints/MyGameMode` (`GameplayStatics.GetGameMode`)))
      (bind _output_get (set `/Game/Blueprints/MyGameMode.Max Lives` (- (`/Game/Blueprints/MyGameMode.Max Lives` _asmy_game_mode) 1) _asmy_game_mode))
      (if (== _output_get 0)
        (bind _returnvalue (`|CreateWidget` "/Game/Widgets/GameOver.GameOver_C"))
        (`UserWidget.AddToViewport` _returnvalue 0)
        (`self.DisableInput` null)
        (`KismetSystemLibrary.Delay` 2.0)
        (`GameplayStatics.OpenLevel` "FirstLevel")))))

(fn `UserConstructionScript`)